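; Interactable button, a child of a parent button Blueprint, that switches the color of a matching BP_ColorSwitch actor as part of an ordered task.
; On Interact it runs the parent logic, then continues only if CheckTaskOrder passes.
; It searches all BP_ColorSwitch actors for the first whose ColorSwitchValue equals its ButtonValue, calls SwitchColor, increments the returned task value and calls GlowIfWrong.
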(event EventInteract
  (params (CharacterRef :type Character%20Object%20Reference))
  (|CallParentFunction CharacterRef)
  (bind (_returnvalue _outputpin) (CallFunction|CheckTaskOrder CharacterRef))
  (if _returnvalue
    (bind _outactors (Actor|GetAllActorsOfClass "/Game/BP/BP_ColorSwitch.BP_ColorSwitch_C"))
    (bind _array_element (Utilities|Array|ForEachLoopwithBreak _outactors :!label _label)
      (:LoopBody
        (if (== (Variables|/Game/BP/BP_ColorSwitch.BP_ColorSwitch_C|GetColorSwitchValue _array_element) (Variables|Default|GetButtonValue))
          (Default|SwitchColor _array_element)
          (Class|PlayerComponent|IncreaseTaskValue _outputpin)
          (CallFunction|GlowifWrong)
          (goto _label Break))))))

(fn ConstructionScript
  (|CallParentFunction))