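; BP_EcranPlat is a flat-screen prop that shows a static screen material until it is triggered to play video.
; On BeginPlay it applies the idle screen material and turns media looping off.
; The ActiveSienna event swaps to the video material once, guarded by a flag, then opens the passed media source on the MediaPlayer on each call.
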(event Custom|Active%20Sienna
  (params (Media%20Source :type Media%20Source%20Object%20Reference))
  (if (Variables|Default|GetIsMatChanged)
    _
    (else
      (Rendering|Material|SetMaterial (Variables|Default|GetFBX_EcranPlat_Ecran) 0 "/Game/Materials/salle_principale/EcranPlat/M_VideoMaterial_Inst.M_VideoMaterial_Inst")
      (Variables|Default|SetIsMatChanged true)))
  (Media|MediaPlayer|OpenSource (Variables|Default|GetMediaPlayer) Media%20Source))

(event EventBeginPlay
  (Rendering|Material|SetMaterial (Variables|Default|GetFBX_EcranPlat_Ecran) 0 "/Game/Materials/salle_principale/EcranPlat/M_EcranPlat_Ecran_Inst.M_EcranPlat_Ecran_Inst")
  (Variables|Default|SetIsMatChanged false)
  (Components|Timeline|SetLooping (Variables|Default|GetMediaPlayer) false))

(fn ConstructionScript)