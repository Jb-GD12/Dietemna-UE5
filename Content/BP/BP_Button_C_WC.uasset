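; Toilet flush button Blueprint that extends a parent interactable with WC-specific behavior.
; On interaction it runs the parent logic, then, if the task order check passes, plays the flush sound, closes the bowl (Cuvette) via animation, increments the task value and calls GlowIfWrong.
; On day 3 it also triggers a player voice line.
; The construction script finds the player and bowl actors by class.
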(event EventInteract
  (params (CharacterRef :type Character%20Object%20Reference))
  (bind _playerref (Variables|Default|GetPlayerRef))
  (|CallParentFunction CharacterRef)
  (bind (_returnvalue _outputpin) (CallFunction|CheckTaskOrder CharacterRef))
  (if _returnvalue
    (CallFunction|PlayWCSound)
    (Default|AnimCloseCuvette (Variables|Default|GetCuvette))
    (Class|PlayerComponent|IncreaseTaskValue _outputpin)
    (CallFunction|GlowifWrong)
    (bind _dayvalue (CallFunction|CheckDay _playerref))
    (if (== _dayvalue 3)
      (Default|Speak _playerref "/Game/Sound/Voices/Jour3/Astute/Voice_Astute_J3_1_Cue.Voice_Astute_J3_1_Cue"))))

(fn ConstructionScript
  (|CallParentFunction)
  (bind _returnvalue (Actor|GetActorOfClass "/Game/BP/FirstPerson/FirstPersonCharacter.FirstPersonCharacter_C"))
  (Variables|Default|SetPlayerRef _returnvalue)
  (bind _returnvalue_2 (Actor|GetActorOfClass "/Game/BP/Bp_CuvetteWC.Bp_CuvetteWC_C"))
  (Variables|Default|SetCuvette _returnvalue_2))

(fn PlayWCSound
  (bind _returnvalue (Audio|SpawnSoundAttached "/Game/Sound/toilette.toilette" (Variables|Default|GetMediaSound) "None" "0, 0, 0" "0, 0, 0" "KeepRelativeOffset" false 1.0 1.0 0.0 "/Game/Sound/TestAttenuation.TestAttenuation" 0))
  (Variables|Default|SetWCSound _returnvalue))

(fn StopWCSound
  (Audio|Components|Audio|Stop (Variables|Default|GetWCSound)))