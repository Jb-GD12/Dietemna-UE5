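; Camera button that, when pressed at a specific player task step, advances the task and fires a scripted scene change.
; The press shifts the main room upward, repositions and flips the cabin, stops the radio hallucination, sounds the alarm clock and shows the camera display.
; After a short delay the player character speaks a voice line and the secret-room spotlights switch and glitch.
; References are cached at BeginPlay and construction; the airlock door unlock is disconnected.
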(event EventBeginPlay
  (bind _returnvalue (Actor|GetActorOfClass "/Game/BP/Screen/DisplayCam.DisplayCam_C"))
  (Variables|Default|SetDisplayCamref _returnvalue)
  (bind _returnvalue_2 (Actor|GetActorOfClass "/Game/BP/BP_Button_C_Radio.BP_Button_C_Radio_C"))
  (Variables|Default|SetRadioRef _returnvalue_2)
  (bind _returnvalue_3 (Actor|GetActorOfClass "/Game/BP/BP_Button_C_AlarmClock.BP_Button_C_AlarmClock_C"))
  (Variables|Default|SetClockRef _returnvalue_3)
  (bind _outactors (Actor|GetAllActorsOfClass "/Game/BP/BP_Door_Sas1_T3.BP_Door_Sas1_T3_C"))
  (for _array_element _outactors
    (if (== (Variables|/Game/BP/BP_Door_Sas1_T3.BP_Door_Sas1_T3_C|GetDoorValue _array_element) 1)
      (Variables|Default|SetSas1 _array_element)
      (else
        (Variables|Default|SetSas2 _array_element)))))

(event EventInteract
  (params (CharacterRef :type Character%20Object%20Reference))
  (bind _returnvalue (Actor|GetComponentbyClass CharacterRef "/Script/Dietemna.PlayerComponent"))
  (|CallParentFunction CharacterRef)
  (bind _returnvalue_2 (Actor|GetActorOfClass "/Game/BP/FirstPerson/FirstPersonCharacter.FirstPersonCharacter_C"))
  (bind _returnvalue_3 (Class|PlayerComponent|GetTaskValue _returnvalue))
  (if (== _returnvalue_3 5)
    (Class|PlayerComponent|IncreaseTaskValue _returnvalue)
    (bind _returnvalue_4 (Actor|GetActorOfClass "/Game/BP/PrefabLD/Modules/olds/MainRoom.MainRoom_C"))
    (bind _output_get (Variables|Default|SetMainRoom _returnvalue_4))
    (Transformation|AddActorWorldOffset _output_get "0, 0,500.000000")
    (Audio|Components|Audio|Stop (Variables|/Game/BP/BP_Button_C_Radio.BP_Button_C_Radio_C|GetRadioHallu (Variables|Default|GetRadioRef)))
    (bind _returnvalue_5 (Actor|GetActorOfClass "/Game/BP/PrefabLD/Modules/CabineJ1.CabineJ1_C"))
    (bind _output_get_2 (Variables|Default|SetCabineRef _returnvalue_5))
    (Transformation|SetActorLocation _output_get_2 "-453.330414,-92.706062,39.855202" false false)
    (Transformation|SetActorRotation _output_get_2 "0,180.000000, 0")
    (Default|PlayAlarmSound (Variables|Default|GetClockRef))
    (Rendering|SetVisibility (Variables|/Game/BP/Screen/DisplayCam.DisplayCam_C|GetWidget (Variables|Default|GetDisplayCamref)) true false)
    (Utilities|FlowControl|Delay 3.0)
    (Default|Speak _returnvalue_2 "/Game/Sound/Voices/Jour6/Astute/Voice_Astute_J6_31_Cue.Voice_Astute_J6_31_Cue")
    (Actor|GetActorOfClass "/Game/BP/Pendu_Blueprint.Pendu_Blueprint_C")
    (for _array_element (Variables|Default|GetSpotSecretRoom)
      (Default|Switch _array_element)
      (Default|LightBug _array_element))))

(fn ConstructionScript
  (|CallParentFunction)
  (bind _outactors (Actor|GetAllActorsOfClass "/Game/BP/Spot_SecretRoom_Blueprint.Spot_SecretRoom_Blueprint_C"))
  (Variables|Default|SetSpotSecretRoom _outactors))