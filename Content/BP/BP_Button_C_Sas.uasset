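; BP_Button_C_Sas is an interactable airlock (Sas) button that opens Sas1 only when the player's task value reaches DayTaskValue and Sas2 is closed.
; Its construction script finds BP_Door_Sas actors, assigning the ButtonValue match to Sas1 and others to Sas2.
; Tick polls the same conditions to set BodyPaint's emissive blue when usable, red otherwise.
; The ChangeColor timeline is never triggered.
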(event EventTick
  (params (DeltaSeconds :type Float%20%28single-precision%29))
  (bind _returnvalue (Class|PlayerComponent|GetTaskValue (Actor|GetComponentbyClass (Game|GetPlayerCharacter 0) "/Script/Dietemna.PlayerComponent")))
  (if (>= _returnvalue (Variables|Default|GetDayTaskValue))
    (if (Variables|/Game/BP/BP_Door_Sas.BP_Door_Sas_C|GetDoorClosed (Variables|Default|GetSas2))
      (Rendering|Material|SetVectorParameterValue (Variables|Default|GetBodyPaint) "EmissiveColor" (Variables|Default|GetMatColorBlue) :!class /Script/Engine.MaterialInstanceDynamic)
      (else
        (Rendering|Material|SetVectorParameterValue (Variables|Default|GetBodyPaint) "EmissiveColor" (Variables|Default|GetMatRedRed) :!class /Script/Engine.MaterialInstanceDynamic :!label _label)))
    (else
      (goto _label))))

(event EventInteract
  (params (CharacterRef :type Character%20Object%20Reference))
  ;[1 1 1] Lock door until player task ok && Open Sas1 if Sas2 closed
  (|CallParentFunction CharacterRef)
  (bind _returnvalue (Class|PlayerComponent|GetTaskValue (Actor|GetComponentbyClass CharacterRef "/Script/Dietemna.PlayerComponent")))
  (if (>= _returnvalue (Variables|Default|GetDayTaskValue))
    (if (Variables|/Game/BP/BP_Door_Sas.BP_Door_Sas_C|GetDoorClosed (Variables|Default|GetSas2))
      (Default|OpenDoor (Variables|Default|GetSas1) CharacterRef))))

(fn ConstructionScript
  (|CallParentFunction)
  (Rendering|Material|SetVectorParameterValue (Variables|Default|GetBodyPaint) "EmissiveColor" (Variables|Default|GetMatColorBlue) :!class /Script/Engine.MaterialInstanceDynamic)
  (bind _outactors (Actor|GetAllActorsOfClass "/Game/BP/BP_Door_Sas.BP_Door_Sas_C"))
  (bind _array_element (Utilities|Array|ForEachLoopwithBreak _outactors)
    (:LoopBody
      (if (== (Variables|/Game/BP/BP_Door_Sas.BP_Door_Sas_C|GetDoorValue _array_element) (Variables|Default|GetButtonValue))
        (Variables|Default|SetSas1 _array_element)
        (else
          (Variables|Default|SetSas2 _array_element))))))