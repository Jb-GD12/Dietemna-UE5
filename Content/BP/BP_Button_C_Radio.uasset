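; Radio button that plays day-specific story audio when the player interacts and reveals the keypad.
; Days 1–3 play radio speeches behind a task-order, one-shot check; days 4–5 stop the static and play computer speech through the Alim button.
; Audio-finished callbacks chain player voice lines or GlowIfWrong, while some days also advance the task.
; BeginPlay starts a Radio Free Cuba sound on days 4 and 6; construction caches actor references.
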(event Custom|AfterDialogue
  (Default|Speak (Variables|Default|GetPlayerRef) "/Game/Sound/Voices/Jour5/Astute/Voice_Astute_J5_2_Cue.Voice_Astute_J5_2_Cue"))

(event Custom|AfterDia
  (CallFunction|GlowifWrong))

(event Custom|CustomEvent
  (CallFunction|GlowifWrong))

(event Custom|AfterDialogue1
  (CallFunction|GlowifWrong))

(event Custom|CustomEvent_0
  (Default|Speak (Variables|Default|GetPlayerRef) "/Game/Sound/Voices/Jour4/Astute/Voice_Astute_J4_2_Cue.Voice_Astute_J4_2_Cue"))

(event EventBeginPlay
  (bind _dayvalue (CallFunction|CheckDay (Game|GetPlayerCharacter 0)))
  (switch int _dayvalue
    (:4
      _)
    (:6
      _))
  (bind _returnvalue (Audio|SpawnSoundAttached "/Game/Sound/Music/RadioFreeCuba_J4_.RadioFreeCuba_J4_" (Variables|Default|GetMediaSound) "None" "0, 0, 0" "0, 0, 0" "KeepRelativeOffset" false 1.0 1.0 0.0 "/Game/Sound/FX/TestAttenuation.TestAttenuation" 0))
  (Variables|J4|SetRadioHallu _returnvalue))

(event EventInteract
  (params (CharacterRef :type Character%20Object%20Reference))
  (bind _alim (Variables|Ref|GetAlim))
  (bind _alim_2 (Variables|Ref|GetAlim))
  (|CallParentFunction CharacterRef)
  (bind (_dayvalue _outputpin) (CallFunction|CheckDay CharacterRef))
  (switch int _dayvalue
    (:1
      (Utilities|CheckTaskandActive CharacterRef)
      (bind _output_get (Variables|Default|SetRadioSpeech (Variables|J1|GetRadioSpeechJ1)))
      (bind _returnvalue (Audio|SpawnSoundAttached _output_get (Variables|Default|GetMediaSound) "None" "0, 0, 0" "0, 0, 0" "KeepRelativeOffset" false 1.0 1.0 0.0 "/Game/Sound/FX/TestAttenuation.TestAttenuation" 0))
      (EventDispatchers|BindEventtoOnAudioFinished _returnvalue (delegate Custom|AfterDialogue1))
      (Rendering|SetVisibility (Variables|/Script/Engine.Actor|GetRootComponent (Variables|Ref|GetKeypad)) true true)
      (Class|PlayerComponent|IncreaseTaskValue _outputpin))
    (:2
      (Utilities|CheckTaskandActive CharacterRef)
      (bind _output_get_2 (Variables|Default|SetRadioSpeech (Variables|J2|GetRadioSpeechJ2)))
      (bind _returnvalue_2 (Audio|SpawnSoundAttached _output_get_2 (Variables|Default|GetMediaSound) "None" "0, 0, 0" "0, 0, 0" "KeepRelativeOffset" false 1.0 1.0 0.0 "/Game/Sound/FX/TestAttenuation.TestAttenuation" 0))
      (EventDispatchers|BindEventtoOnAudioFinished _returnvalue_2 (delegate Custom|AfterDia))
      (Utilities|FlowControl|Delay 1.0)
      (Default|Speak (Variables|Default|GetPlayerRef) "/Game/Sound/Voices/Jour2/Astute/Voice_Astute_J2_5_Cue.Voice_Astute_J2_5_Cue")
      (Rendering|SetVisibility (Variables|/Script/Engine.Actor|GetRootComponent (Variables|Ref|GetKeypad)) true true))
    (:3
      (Utilities|CheckTaskandActive CharacterRef)
      (bind _output_get_3 (Variables|Default|SetRadioSpeech (Variables|J3|GetRadioSpeechJ3)))
      (bind _returnvalue_3 (Audio|SpawnSoundAttached _output_get_3 (Variables|Default|GetMediaSound) "None" "0, 0, 0" "0, 0, 0" "KeepRelativeOffset" false 1.0 1.0 0.0 "/Game/Sound/FX/TestAttenuation.TestAttenuation" 0))
      (EventDispatchers|BindEventtoOnAudioFinished _returnvalue_3 (delegate Custom|CustomEvent))
      (Utilities|FlowControl|Delay 1.0)
      (Default|Speak (Variables|Default|GetPlayerRef) "/Game/Sound/Voices/Jour3/Astute/Voice_Astute_J3_3_Cue.Voice_Astute_J3_3_Cue")
      (Rendering|SetVisibility (Variables|/Script/Engine.Actor|GetRootComponent (Variables|Ref|GetKeypad)) true true))
    (:4
      (bind (_returnvalue_4 _outputpin_2) (CallFunction|CheckTaskOrder CharacterRef))
      (if _returnvalue_4
        (bind _returnvalue_5 (Audio|SpawnSoundAttached (Variables|/Game/BP/BP_Button_C_Alim.BP_Button_C_Alim_C|GetComputerSpeechJ4 _alim_2) (Actor|GetComponentbyClass _alim_2 "/Script/MediaAssets.MediaSoundComponent") "None" "0, 0, 0" "0, 0, 0" "KeepRelativeOffset" false 1.0 1.0 0.0 "/Game/Sound/FX/TestAttenuation.TestAttenuation" 0))
        (bind _output_get_4 (Variables|/Game/BP/BP_Button_C_Alim.BP_Button_C_Alim_C|SetJ4GlitchSpeech _alim_2 _returnvalue_5))
        (EventDispatchers|BindEventtoOnAudioFinished _output_get_4 (delegate Custom|CustomEvent_0))
        (Audio|Components|Audio|Stop (Variables|J4|GetRadioNeige))
        (Class|PlayerComponent|IncreaseTaskValue _outputpin_2)
        (CallFunction|GlowifWrong)
        (Rendering|SetVisibility (Variables|/Script/Engine.Actor|GetRootComponent (Variables|Ref|GetKeypad)) true true)))
    (:5
      (bind (_returnvalue_6 _outputpin_3) (CallFunction|CheckTaskOrder CharacterRef))
      (if _returnvalue_6
        (bind _returnvalue_7 (Audio|SpawnSoundAttached (Variables|/Game/BP/BP_Button_C_Alim.BP_Button_C_Alim_C|GetComputerSpeechJ5 _alim) (Actor|GetComponentbyClass _alim "/Script/MediaAssets.MediaSoundComponent") "None" "0, 0, 0" "0, 0, 0" "KeepRelativeOffset" false 1.0 1.0 0.0 "/Game/Sound/FX/TestAttenuation.TestAttenuation" 0))
        (EventDispatchers|BindEventtoOnAudioFinished _returnvalue_7 (delegate Custom|AfterDialogue))
        (Audio|Components|Audio|Stop (Variables|J4|GetRadioNeige))
        (Class|PlayerComponent|IncreaseTaskValue _outputpin_3)
        (CallFunction|GlowifWrong)
        (Rendering|SetVisibility (Variables|/Script/Engine.Actor|GetRootComponent (Variables|Ref|GetKeypad)) true true)))))

(fn ConstructionScript
  (|CallParentFunction)
  (bind _returnvalue (Actor|GetActorOfClass "/Game/BP/Puzzle/BP_Keypad_Com.BP_Keypad_Com_C"))
  (Variables|Ref|SetKeypad _returnvalue)
  (bind _returnvalue_2 (Actor|GetActorOfClass "/Game/BP/BP_Button_C_Alim.BP_Button_C_Alim_C"))
  (Variables|Ref|SetAlim _returnvalue_2)
  (bind _returnvalue_3 (Actor|GetActorOfClass "/Game/BP/FirstPerson/FirstPersonCharacter.FirstPersonCharacter_C"))
  (Variables|Default|SetPlayerRef _returnvalue_3))