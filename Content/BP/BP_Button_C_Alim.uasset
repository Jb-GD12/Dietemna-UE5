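; Interactable "Alim" button (apparently the power switch) that drives a story task, varying by in-game day.
; Days 1–3 gate on task order and a one-shot flag, play computer speech and advance the task when it finishes; days 1–2 also switch on all lights.
; Day 2 starts with an alarm that the press silences.
; Days 4–5 start the radio speech and advance the task immediately.
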(event Custom|AfterDialogue2
  ;[1 1 1] Jour 2
  (Class|PlayerComponent|IncreaseTaskValue (Variables|Default|GetPlayerCompRef))
  (CallFunction|GlowifWrong))

(event Custom|AfterDiag2
  (Audio|SpawnSoundAttached "/Game/Sound/Voices/Jour1/Sienna/Voice_Sienna_J0_3.Voice_Sienna_J0_3" (Variables|Default|GetMediaSound) "None" "0, 0, 0" "0, 0, 0" "KeepRelativeOffset" false 1.0 1.0 0.0 "/Game/Sound/TestAttenuation.TestAttenuation" 0))

(event Custom|AfterDialogue3
  ;[1 1 1] Jour 3
  (Class|PlayerComponent|IncreaseTaskValue (Variables|Default|GetPlayerCompRef))
  (CallFunction|GlowifWrong))

(event Custom|AfterDialogue1
  ;[1 1 1] Jour 1
  (Class|PlayerComponent|IncreaseTaskValue (Variables|Default|GetPlayerCompRef))
  (CallFunction|GlowifWrong)
  (bind _returnvalue (Audio|SpawnSoundAttached "/Game/Sound/Voices/Jour1/Sienna/Voice_Sienna_J0_2.Voice_Sienna_J0_2" (Variables|Default|GetMediaSound) "None" "0, 0, 0" "0, 0, 0" "KeepRelativeOffset" false 1.0 1.0 0.0 "/Game/Sound/TestAttenuation.TestAttenuation" 0))
  (EventDispatchers|BindEventtoOnAudioFinished _returnvalue (delegate Custom|AfterDiag2)))

(event EventBeginPlay
  (bind _dayvalue (CallFunction|CheckDay (Game|GetPlayerCharacter 0)))
  (if (== _dayvalue 2)
    (bind _returnvalue (Audio|SpawnSoundAttached (Variables|J2|GetAlarmJ2) (Variables|Default|GetMediaSound) "None" "0, 0, 0" "0, 0, 0" "KeepRelativeOffset" false 1.0 1.0 0.0 "/Game/Sound/TestAttenuation1.TestAttenuation1" 0))))

(event EventInteract
  (params (CharacterRef :type Character%20Object%20Reference))
  (bind _radio (Variables|Ref|GetRadio))
  (bind _radio_2 (Variables|Ref|GetRadio))
  (|CallParentFunction CharacterRef)
  (bind (_dayvalue _outputpin) (CallFunction|CheckDay CharacterRef))
  (Variables|Default|SetPlayerCompRef _outputpin)
  (switch int _dayvalue
    (:1
      ;[1 1 1] Jour 1
      (Utilities|CheckTaskandActive CharacterRef)
      (bind _array_element (Utilities|Array|ForEachLoopwithBreak (Variables|Default|GetAllLights))
        (:LoopBody
          (Default|SwitchonLight _array_element))
        (:Completed
          (bind _returnvalue (Audio|SpawnSoundAttached (Variables|J1|GetComputerSpeechJ1) (Variables|Default|GetMediaSound) "None" "0, 0, 0" "0, 0, 0" "KeepRelativeOffset" false 1.0 1.0 0.0 "/Game/Sound/TestAttenuation.TestAttenuation" 0))
          (EventDispatchers|BindEventtoOnAudioFinished _returnvalue (delegate Custom|AfterDialogue1))
          (Utilities|FlowControl|Delay 1.0)
          (Default|Speak (Variables|Default|GetPlayerRef) "/Game/Sound/Voices/Jour1/Astute/Voice_Astute_J1_1_Cue.Voice_Astute_J1_1_Cue"))))
    (:2
      ;[1 1 1] Jour 2
      (Utilities|CheckTaskandActive CharacterRef)
      (Audio|Components|Audio|Stop (stale EventBeginPlay _returnvalue))
      (bind _array_element_2 (Utilities|Array|ForEachLoopwithBreak (Variables|Default|GetAllLights))
        (:LoopBody
          (Default|SwitchonLight _array_element_2))
        (:Completed
          (bind _returnvalue_2 (Audio|SpawnSoundAttached (Variables|J2|GetComputerSpeechJ2) (Variables|Default|GetMediaSound) "None" "0, 0, 0" "0, 0, 0" "KeepRelativeOffset" false 1.0 1.0 0.0 "/Game/Sound/TestAttenuation.TestAttenuation" 0))
          (EventDispatchers|BindEventtoOnAudioFinished _returnvalue_2 (delegate Custom|AfterDialogue2)))))
    (:3
      ;[1 1 1] Jour 3
      (Utilities|CheckTaskandActive CharacterRef)
      (bind _returnvalue_3 (Audio|SpawnSoundAttached (Variables|J3|GetComputerSpeechJ3) (Variables|Default|GetMediaSound) "None" "0, 0, 0" "0, 0, 0" "KeepRelativeOffset" false 1.0 1.0 0.0 "/Game/Sound/TestAttenuation.TestAttenuation" 0))
      (EventDispatchers|BindEventtoOnAudioFinished _returnvalue_3 (delegate Custom|AfterDialogue3)))
    (:4
      ;[1 1 1] Jour 4
      (bind _returnvalue_4 (CallFunction|CheckTaskOrder CharacterRef))
      (if _returnvalue_4
        (bind _returnvalue_5 (Audio|SpawnSoundAttached (Variables|/Game/BP/BP_Button_C_Radio.BP_Button_C_Radio_C|GetRadioSpeechJ4 _radio_2) (Actor|GetComponentbyClass _radio_2 "/Script/MediaAssets.MediaSoundComponent") "None" "0, 0, 0" "0, 0, 0" "KeepRelativeOffset" false 1.0 1.0 0.0 "/Game/Sound/TestAttenuation.TestAttenuation" 0))
        (Variables|/Game/BP/BP_Button_C_Radio.BP_Button_C_Radio_C|SetRadioNeige (Variables|Ref|GetRadio) _returnvalue_5)
        (Class|PlayerComponent|IncreaseTaskValue (Variables|Default|GetPlayerCompRef))
        (CallFunction|GlowifWrong)))
    (:5
      ;[1 1 1] Jour 5
      (bind _returnvalue_6 (CallFunction|CheckTaskOrder CharacterRef))
      (if _returnvalue_6
        (bind _returnvalue_7 (Audio|SpawnSoundAttached (Variables|/Game/BP/BP_Button_C_Radio.BP_Button_C_Radio_C|GetRadioSpeechJ4 _radio) (Actor|GetComponentbyClass _radio "/Script/MediaAssets.MediaSoundComponent") "None" "0, 0, 0" "0, 0, 0" "KeepRelativeOffset" false 1.0 1.0 0.0 "/Game/Sound/TestAttenuation.TestAttenuation" 0))
        (Variables|/Game/BP/BP_Button_C_Radio.BP_Button_C_Radio_C|SetRadioNeige (Variables|Ref|GetRadio) _returnvalue_7)
        (Class|PlayerComponent|IncreaseTaskValue (Variables|Default|GetPlayerCompRef))
        (CallFunction|GlowifWrong)))))

(fn ConstructionScript
  (|CallParentFunction)
  (bind _outactors (Actor|GetAllActorsOfClass "/Game/BP/BP_Lights.BP_Lights_C"))
  (Variables|Default|SetAllLights _outactors)
  (bind _returnvalue (Actor|GetActorOfClass "/Game/BP/BP_Button_C_Radio.BP_Button_C_Radio_C"))
  (Variables|Ref|SetRadio _returnvalue)
  (bind _returnvalue_2 (Actor|GetActorOfClass "/Game/BP/FirstPerson/FirstPersonCharacter.FirstPersonCharacter_C"))
  (Variables|Default|SetPlayerRef _returnvalue_2))