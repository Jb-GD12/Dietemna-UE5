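; BP_Button_C_Door is a button child Blueprint that opens its matching interactive door when a character interacts with it in the correct task order.
; After the parent interaction runs and the task order check passes, it searches all BP_Door_Interact actors for a DoorValue equal to its ButtonValue.
; The first match opens, then the task value increases and GlowIfWrong runs.
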(event EventInteract
  (params (CharacterRef :type Character%20Object%20Reference))
  (|CallParentFunction CharacterRef)
  (bind (_returnvalue _outputpin) (CallFunction|CheckTaskOrder CharacterRef))
  (if _returnvalue
    (bind _outactors (Actor|GetAllActorsOfClass "/Game/BP/BP_Door_Interact.BP_Door_Interact_C"))
    (bind _array_element (Utilities|Array|ForEachLoopwithBreak _outactors :!label _label)
      (:LoopBody
        (if (== (Variables|/Game/BP/BP_Door_Interact.BP_Door_Interact_C|GetDoorValue _array_element) (Variables|Default|GetButtonValue))
          (Default|OpenDoor _array_element CharacterRef)
          (Class|PlayerComponent|IncreaseTaskValue _outputpin)
          (CallFunction|GlowifWrong)
          (goto _label Break))))))

(fn ConstructionScript
  (|CallParentFunction))