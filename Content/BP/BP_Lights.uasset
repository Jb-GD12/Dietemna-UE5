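; BP_Lights is a rect light actor that acts as a fading alarm on day 2 and can switch color.
; On BeginPlay it reads the day from the player's PlayerComponent and starts a timeline pulsing intensity, replayed in reverse while NotActive holds.
; SwitchOnLight alternately plays a color timeline forward and backward; its completion clears NotActive, ending the pulse at fixed brightness.
; The construction script applies the Intensity variable.
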(event Custom|SwitchOnLight
  (Utilities|FlowControl|FlipFlop
    (:A
      ;[1 1 1] Change Light color
      (bind _lightlinearcolortrack (Timeline|LightTimeline PlayFromStart)
        (:Update
          (Rendering|Components|Light|SetLightColor (Variables|Default|GetRectLight) _lightlinearcolortrack true))
        (:Finished
          (Variables|Default|SetNotActive false))))
    (:B
      (Timeline|LightTimeline ReverseFromEnd))))

(event EventBeginPlay
  (bind _rectlight (Variables|Default|GetRectLight))
  (bind _returnvalue (Class|PlayerComponent|GetDayValue (Actor|GetComponentbyClass (Game|GetPlayerCharacter 0) "/Script/Dietemna.PlayerComponent")))
  ;[1 1 1] Fading Light Alarm only J2
  (if (== _returnvalue 2)
    (bind _lightbrightnessfloattrack (Timeline|FadingLight PlayFromStart)
      (:Update
        (if (Variables|Default|GetNotActive)
          (Rendering|Components|Light|SetIntensity _rectlight (* _lightbrightnessfloattrack 5e+03))
          (else
            (Rendering|Components|Light|SetIntensity _rectlight 5e+03))))
      (:Finished
        (if (Variables|Default|GetNotActive)
          (Timeline|FadingLight ReverseFromEnd))))))

(fn ConstructionScript
  (Rendering|Components|Light|SetIntensity (Variables|Default|GetRectLight) (Variables|Light|GetIntensity)))