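; Interactive sink valve that toggles between turned and unturned each time it receives an Interact event.
; A FlipFlop plays the RotZ timeline forward or in reverse, driving the Valve's relative yaw by the curve value scaled to degrees.
; When the timeline finishes, the FlipFlop state selects a French debug print standing in for spawning or destroying the water instance, which is not implemented here.
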(event EventInteract
  (params (CharacterRef :type Character%20Object%20Reference))
  (bind _valve (Variables|Default|GetValve))
  (bind _relativerotation (Variables|/Script/Engine.SceneComponent|GetRelativeRotation _valve))
  (bind (_roll _pitch) (Math|Rotator|BreakRotator _relativerotation))
  (bind _isa (Utilities|FlowControl|FlipFlop)
    (:A
      (bind _rotz (Timeline|RotZ PlayFromStart)
        (:Update
          (Transformation|SetRelativeRotation _valve (Math|Rotator|MakeRotator _roll _pitch (* _rotz 6e+01)) false false))
        (:Finished
          (if _isa
            (Development|PrintString "SPAWN TON INSTANCE DE LEAU")
            (else
              (Development|PrintString "DESTROY TON INSTANCE DE LEAU"))))))
    (:B
      (Timeline|RotZ ReverseFromEnd))))

(fn ConstructionScript)