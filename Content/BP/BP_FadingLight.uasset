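; BP_FadingLight is a point light that fades in when something overlaps its collision and fades back out when the overlap ends.
; A timeline plays from the start on begin overlap and reverses on end overlap, driving color and multiplier-scaled intensity.
; The construction script sets intensity to zero so the light starts dark.
; Overlaps are not filtered by actor, and a debug print is left unconnected.
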(event OnComponentBeginOverlap(OverlapCollision)
  (params (OverlappedComponent :type Primitive%20Component%20Object%20Reference) (OtherActor :type Actor%20Object%20Reference) (OtherComp :type Primitive%20Component%20Object%20Reference) (OtherBodyIndex :type Integer) (bFromSweep :type Boolean) (SweepResult :type Hit%20Result%20Structure%20%28by%20ref%29))
  (bind _pointlight (Variables|Components|GetPointLight))
  ;[1 1 1] Fading Light
  (bind (_direction _lightbrightnessfloattrack _lightlinearcolortrack) (Timeline|PointLightTimeline PlayFromStart)
    (:Update
      (Rendering|Components|Light|SetIntensity _pointlight (* _lightbrightnessfloattrack (Variables|Light|GetBrightnessMultiplier)))
      (Rendering|Components|Light|SetLightColor _pointlight _lightlinearcolortrack true))))

(event OnComponentEndOverlap(OverlapCollision)
  (params (OverlappedComponent :type Primitive%20Component%20Object%20Reference) (OtherActor :type Actor%20Object%20Reference) (OtherComp :type Primitive%20Component%20Object%20Reference) (OtherBodyIndex :type Integer))
  (bind _pointlight (Variables|Components|GetPointLight))
  ;[1 1 1] Fading Light
  (bind (_direction _lightbrightnessfloattrack _lightlinearcolortrack) (Timeline|PointLightTimeline Reverse)
    (:Update
      (Rendering|Components|Light|SetIntensity _pointlight (* _lightbrightnessfloattrack (Variables|Light|GetBrightnessMultiplier)))
      (Rendering|Components|Light|SetLightColor _pointlight _lightlinearcolortrack true))))

(fn ConstructionScript
  (Rendering|Components|Light|SetIntensity (Variables|Components|GetPointLight) 0.0))