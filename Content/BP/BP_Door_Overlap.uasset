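; Door Blueprint that swings open when an actor enters its overlap volume and closes when an overlap ends.
; A timeline scales the Door component's relative yaw up to 90 degrees, playing on begin overlap and reversing on end overlap.
; The sign of the overlapping actor's world-space forward X picks the swing direction, without accounting for the door's own orientation.
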(event OnComponentBeginOverlap(OpeningOverlap)
  (params (OverlappedComponent :type Primitive%20Component%20Object%20Reference) (OtherActor :type Actor%20Object%20Reference) (OtherComp :type Primitive%20Component%20Object%20Reference) (OtherBodyIndex :type Integer) (bFromSweep :type Boolean) (SweepResult :type Hit%20Result%20Structure%20%28by%20ref%29))
  (Variables|Default|SetForwardVect (Transformation|GetActorForwardVector OtherActor))
  (bind _doorrotationz (Timeline|DoorTimelineComponent Play)
    (:Update
      (if (< (.X (Math|Vector|BreakVector (Variables|Default|GetForwardVect))) 0.0)
        ;[1 1 1] Rotate Door -90°
        (Transformation|SetRelativeRotation (Variables|Default|GetDoor) (Math|Rotator|MakeRotator 0.0 0.0 (* (* _doorrotationz 9e+01) -1.0)) false false)
        (else
          ;[1 1 1] Rotate Door +90°
          (Transformation|SetRelativeRotation (Variables|Default|GetDoor) (Math|Rotator|MakeRotator 0.0 0.0 (* _doorrotationz 9e+01)) false false))))))

(event OnComponentEndOverlap(OpeningOverlap)
  (params (OverlappedComponent :type Primitive%20Component%20Object%20Reference) (OtherActor :type Actor%20Object%20Reference) (OtherComp :type Primitive%20Component%20Object%20Reference) (OtherBodyIndex :type Integer))
  (bind _doorrotationz (Timeline|DoorTimelineComponent Reverse)
    (:Update
      (if (< (.X (Math|Vector|BreakVector (Variables|Default|GetForwardVect))) 0.0)
        ;[1 1 1] Rotate Door -90°
        (Transformation|SetRelativeRotation (Variables|Default|GetDoor) (Math|Rotator|MakeRotator 0.0 0.0 (* (* _doorrotationz 9e+01) -1.0)) false false)
        (else
          ;[1 1 1] Rotate Door +90°
          (Transformation|SetRelativeRotation (Variables|Default|GetDoor) (Math|Rotator|MakeRotator 0.0 0.0 (* _doorrotationz 9e+01)) false false))))))

(fn ConstructionScript)