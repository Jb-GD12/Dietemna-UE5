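; Valve interactable that opens one of two interlocked airlock (sas) doors, selected by ButtonValue, once the player's task value reaches DayTaskValue.
; A door opens only while the other is closed; if it is closed too, a timeline spins the valve before calling OpenDoor.
; Construction finds both doors by class and creates the indicator's dynamic material.
; Tick turns the indicator blue when opening is allowed, red otherwise.
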(event EventTick
  (params (DeltaSeconds :type Float%20%28single-precision%29))
  (bind _returnvalue (Class|PlayerComponent|GetTaskValue (Actor|GetComponentbyClass (Game|GetPlayerCharacter 0) "/Script/Dietemna.PlayerComponent")))
  (if (>= _returnvalue (Variables|Default|GetDayTaskValue))
    (if (== (Variables|Default|GetButtonValue) 1)
      (if (Variables|/Game/BP/BP_Door_Sas2.BP_Door_Sas2_C|GetDoorClosed (Variables|Default|GetSas2))
        (Rendering|Material|SetVectorParameterValue (Variables|Default|GetBodyPaint) "EmissiveColor" (Variables|Default|GetMatColorBlue) :!class /Script/Engine.MaterialInstanceDynamic :!label _label)
        (else
          (Rendering|Material|SetVectorParameterValue (Variables|Default|GetBodyPaint) "EmissiveColor" (Variables|Default|GetMatRedRed) :!class /Script/Engine.MaterialInstanceDynamic :!label _label_2)))
      (elif (Variables|/Game/BP/BP_Door_Sas1_T3.BP_Door_Sas1_T3_C|GetDoorClosed (Variables|Default|GetSas1))
        (goto _label)
        (else
          (goto _label_2))))
    (else
      (goto _label_2))))

(event EventInteract
  (params (CharacterRef :type Character%20Object%20Reference))
  (bind _returnvalue (Class|PlayerComponent|GetTaskValue (Actor|GetComponentbyClass CharacterRef "/Script/Dietemna.PlayerComponent")))
  (if (>= _returnvalue (Variables|Default|GetDayTaskValue))
    (if (== (Variables|Default|GetButtonValue) 1)
      (|OpenSas1 CharacterRef)
      (else
        (|OpenSas2 CharacterRef)))))

(fn ConstructionScript
  (bind _returnvalue (Rendering|Material|CreateDynamicMaterialInstance "/Game/Materials/oldMats/M_buttonOutline_Inst.M_buttonOutline_Inst" "None" "None" :!class /Script/Engine.KismetMaterialLibrary))
  (bind _output_get (Variables|Default|SetBodypaint _returnvalue))
  (Rendering|Material|SetMaterial (Variables|Default|GetTémoinLum) 0 _output_get)
  (Rendering|Material|SetVectorParameterValue (Variables|Default|GetBodyPaint) "EmissiveColor" (Variables|Default|GetMatColorBlue) :!class /Script/Engine.MaterialInstanceDynamic)
  (bind _returnvalue_2 (Actor|GetActorOfClass "/Game/BP/BP_Door_Sas1_T3.BP_Door_Sas1_T3_C"))
  (Variables|Default|SetSas1 _returnvalue_2)
  (bind _returnvalue_3 (Actor|GetActorOfClass "/Game/BP/BP_Door_Sas2.BP_Door_Sas2_C"))
  (Variables|Default|SetSas2 _returnvalue_3))