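; Point light Blueprint for cabin or main-room lighting, with a switchable color and a fading alarm on day 2.
; The construction script sets intensity and the initial color chosen by the Cabine flag.
; SwitchOnLight flip-flops a color timeline forward and backward, though cabin lights keep their initial color.
; On day 2, read from PlayerComponent at BeginPlay, a second timeline repeatedly fades brightness until a finished color timeline clears NotActive.
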(event Custom|SwitchOnLight
  (bind _pointlight (Variables|Default|GetPointLight))
  (Utilities|FlowControl|FlipFlop
    (:A
      ;[1 1 1] Change Light color
      (bind _lightlinearcolortrack (Timeline|LightTimeline PlayFromStart)
        (:Update
          (if (Variables|Default|GetbCabine)
            (Rendering|Components|Light|SetLightColor _pointlight (Variables|Default|GetColorCabineInit) true)
            (else
              (Rendering|Components|Light|SetLightColor _pointlight _lightlinearcolortrack true))))
        (:Finished
          (Variables|Default|SetNotActive false))))
    (:B
      (Timeline|LightTimeline ReverseFromEnd))))

(event EventBeginPlay
  (bind _pointlight (Variables|Default|GetPointLight))
  (bind _returnvalue (Class|PlayerComponent|GetDayValue (Actor|GetComponentbyClass (Game|GetPlayerCharacter 0) "/Script/Dietemna.PlayerComponent")))
  ;[1 1 1] Fading Light Alarm only J2
  (if (== _returnvalue 2)
    (bind _lightbrightnessfloattrack (Timeline|FadingLight PlayFromStart)
      (:Update
        (if (Variables|Default|GetNotActive)
          (Rendering|Components|Light|SetIntensity _pointlight (* _lightbrightnessfloattrack 5e+03))
          (else
            (Rendering|Components|Light|SetIntensity _pointlight 5e+03))))
      (:Finished
        (if (Variables|Default|GetNotActive)
          (Timeline|FadingLight ReverseFromEnd))))))

(fn ConstructionScript
  (bind _pointlight (Variables|Default|GetPointLight))
  (Rendering|Components|Light|SetIntensity _pointlight (Variables|Light|GetIntensity))
  (if (Variables|Default|GetbCabine)
    (Rendering|Components|Light|SetLightColor _pointlight (Variables|Default|GetColorCabineInit) true)
    (else
      (Rendering|Components|Light|SetLightColor _pointlight (Variables|Default|GetColorMainRoomInit) true))))