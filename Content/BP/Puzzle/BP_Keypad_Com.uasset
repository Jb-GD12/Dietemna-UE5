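; Puzzle keypad actor that checks codes entered on its WB_Keypad_Com widget against a correct code and plays success or failure sounds.
; A correct code advances the player's task value through PlayerComponent, but only when the current task matches the keypad's.
; On day 2 that advance also plays a Sienna voice line from the BP_Button_C_Alim actor, then the player's Astute reply.
; The construction script finds both actor references by class.
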(event Custom|CheckCode
  (params (Code :type String) (Keypad :type WB%20Keypad%20Com%20Object%20Reference))
  (bind _returnvalue (Game|GetPlayerCharacter 0))
  (bind _returnvalue_2 (Actor|GetComponentbyClass _returnvalue "/Script/Dietemna.PlayerComponent"))
  (if (Utilities|Enum|Equal(Enum) Code (Variables|Default|GetCorrectCode))
    (Utilities|FlowControl|Delay 0.2)
    (Audio|SpawnSoundAttached (Variables|Default|GetWinPuzzleSound) (Variables|Default|GetMediaSound) "None" "0, 0, 0" "0, 0, 0" "KeepRelativeOffset" false 1.0 1.0 0.0 "/Game/Sound/TestAttenuation.TestAttenuation" 0)
    (bind _returnvalue_3 (Class|PlayerComponent|GetTaskValue _returnvalue_2))
    (if (== (Variables|Default|GetTaskValue) _returnvalue_3)
      (Class|PlayerComponent|IncreaseTaskValue _returnvalue_2)
      (bind _returnvalue_4 (Class|PlayerComponent|GetDayValue _returnvalue_2))
      (if (== _returnvalue_4 2)
        (bind _returnvalue_5 (Audio|SpawnSoundAttached "/Game/Sound/Voices/Jour2/Sienna/Voice_Sienna_J1_3.Voice_Sienna_J1_3" (Variables|/Game/BP/BP_Button_Parent.BP_Button_Parent_C|GetMediaSound (Variables|Default|GetAlimRef)) "None" "0, 0, 0" "0, 0, 0" "KeepRelativeOffset" false 1.0 1.0 0.0 0 0))
        (EventDispatchers|BindEventtoOnAudioFinished _returnvalue_5 (delegate Custom|CustomEvent_0))))
    (else
      (Utilities|FlowControl|Delay 0.2)
      (Audio|SpawnSoundAttached (Variables|Default|GetFailPuzzleSound) (Variables|Default|GetMediaSound) "None" "0, 0, 0" "0, 0, 0" "KeepRelativeOffset" false 1.0 1.0 0.0 "/Game/Sound/TestAttenuation.TestAttenuation" 0))))

(event Custom|CustomEvent_0
  (Default|Speak (Variables|Default|GetPlayerRef) "/Game/Sound/Voices/Jour2/Astute/Voice_Astute_J2_6_Cue.Voice_Astute_J2_6_Cue"))

(event EventBeginPlay
  (bind _aswb_keypad_com (Utilities|Casting|CastToWB_Keypad_Com (UserInterface|GetUserWidgetObject (Variables|Default|GetKeypadWidget))))
  (bind _output_get (Variables|Default|SetKeyPad_Com _aswb_keypad_com))
  (EventDispatchers|BindEventtoCodeEntered _output_get (delegate Custom|CheckCode)))

(fn ConstructionScript
  (Rendering|SetVisibility (Variables|Default|GetDefaultSceneRoot) true true)
  (bind _returnvalue (Actor|GetActorOfClass "/Game/BP/BP_Button_C_Alim.BP_Button_C_Alim_C"))
  (Variables|Default|SetAlimRef _returnvalue)
  (bind _returnvalue_2 (Actor|GetActorOfClass "/Game/BP/FirstPerson/FirstPersonCharacter.FirstPersonCharacter_C"))
  (Variables|Default|SetPlayerRef _returnvalue_2))