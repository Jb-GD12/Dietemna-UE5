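; BP_SoundEmitter is an actor that plays a day-specific sound effect.
; On BeginPlay it reads the day value from the player character's PlayerComponent and switches on it, playing an accident, metal impact or knocking sound on certain days.
; The sound is spawned attached to MediaSound, some with custom attenuation, and stored in SoundInstance so StopSound can stop it later.
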(event EventBeginPlay
  (bind _returnvalue (Class|PlayerComponent|GetDayValue (Actor|GetComponentbyClass (Game|GetPlayerCharacter 0) "/Script/Dietemna.PlayerComponent")))
  (switch int _returnvalue
    (:2
      (bind _returnvalue_2 (Audio|SpawnSoundAttached (Variables|Default|GetAccidentSound) (Variables|Default|GetMediaSound) "None" "0, 0, 0" "0, 0, 0" "KeepRelativeOffset" false 1.0 1.0 0.0 0 0))
      (Variables|Default|SetSoundInstance _returnvalue_2))
    (:4
      (bind _returnvalue_3 (Audio|SpawnSoundAttached "/Game/Sound/MetalImpact.MetalImpact" (Variables|Default|GetMediaSound) "None" "0, 0, 0" "0, 0, 0" "KeepRelativeOffset" false 1.0 1.0 0.0 "/Game/Sound/TestAttenuation.TestAttenuation" 0 :!label _label))
      (Variables|Default|SetSoundInstance _returnvalue_3))
    (:5
      (goto _label))
    (:7
      (bind _returnvalue_4 (Audio|SpawnSoundAttached "/Game/Sound/Knocking-On-Metal-Sound-Effect-Free-Download-HD.Knocking-On-Metal-Sound-Effect-Free-Download-HD" (Variables|Default|GetMediaSound) "None" "0, 0, 0" "0, 0, 0" "KeepRelativeOffset" false 1.0 1.0 0.0 "/Game/Sound/TestAttenuation.TestAttenuation" 0))
      (Variables|Default|SetSoundInstance _returnvalue_4))))

(fn ConstructionScript)

(fn StopSound
  (Audio|Components|Audio|Stop (Variables|Default|GetSoundInstance)))