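; Parent Blueprint for an interactable crank that advances the player's daily task sequence.
; Interact checks PlayerComponent task order, then plays a motor sound and a day-specific rotation timeline.
; After the day's required turn count it increments the task; day 2 first chains two voice lines, day 6 offsets two cabin actors vertically.
; GlowIfWrong drives a dynamic outline material's emissive colour by timeline to show whether the task is done.
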(event Custom|GlowIfWrong
  ;[1 1 1] Glow passe du vert au rouge quand la tâche à été effectué
  (bind _returnvalue (CallFunction|CheckTaskAbove (Game|GetPlayerCharacter 0)))
  (if _returnvalue
    (bind _matcolor (Timeline|Glow2 ReverseFromEnd)
      (:Update
        (Rendering|Material|SetVectorParameterValue (Variables|Default|GetBodyPaint) "EmissiveColor" _matcolor :!class /Script/Engine.MaterialInstanceDynamic)))
    (else
      (Timeline|Glow2 PlayFromStart))))

(event Custom|CustomEvent_0
  (bind _returnvalue (Audio|SpawnSoundAttached "/Game/Sound/Voices/Jour2/Sienna/Voice_Sienna_J1_2.Voice_Sienna_J1_2" (Variables|/Game/BP/BP_Button_Parent.BP_Button_Parent_C|GetMediaSound (Variables|Ref|GetAlimRef)) "None" "0, 0, 0" "0, 0, 0" "KeepRelativeOffset" false 1.0 1.0 0.0 0 0))
  (EventDispatchers|BindEventtoOnAudioFinished _returnvalue (delegate Custom|CustomEvent_1)))

(event Custom|CustomEvent_1
  (Class|PlayerComponent|IncreaseTaskValue (stale EventInteract _outputpin))
  (CallFunction|GlowifWrong))

(event EventBeginPlay
  (CallFunction|GlowifWrong))

(event EventInteract
  (params (CharacterRef :type Character%20Object%20Reference))
  (bind _manivelle_parent (Variables|Default|GetManivelle_parent))
  (bind _manivelle_parent_2 (Variables|Default|GetManivelle_parent))
  (bind _relativerotation (Variables|/Script/Engine.SceneComponent|GetRelativeRotation _manivelle_parent))
  (bind _relativerotation_2 (Variables|/Script/Engine.SceneComponent|GetRelativeRotation _manivelle_parent_2))
  (bind (_roll _pitch _yaw) (Math|Rotator|BreakRotator _relativerotation))
  (bind (_roll_2 _pitch_2 _yaw_2) (Math|Rotator|BreakRotator _relativerotation_2))
  (bind _returnvalue (CallFunction|CheckTaskOrder CharacterRef))
  (if (and _returnvalue (Variables|Default|GetNotInAction))
    (Variables|Default|SetNotInAction false)
    (bind (_dayvalue _outputpin) (CallFunction|CheckDay CharacterRef))
    (switch int _dayvalue
      (:1
        ;[1 1 1] Jour 1
        (Audio|SpawnSoundAttached "/Game/Sound/Motor.Motor" (Variables|Default|GetMediaSound) "None" "0, 0, 0" "0, 0, 0" "KeepRelativeOffset" false 1.0 1.0 0.0 "/Game/Sound/TestAttenuation.TestAttenuation" 0)
        (bind _displacement (Timeline|Interact_anim PlayFromStart)
          (:Update
            (Transformation|SetRelativeRotation (Variables|Default|GetManivelle_parent) (Math|Rotator|MakeRotator _roll _displacement _yaw) false false)
            (Utilities|FlowControl|DoOnce false
              (:Completed
                (Variables|Default|SetTryNumberForNext 1))))
          (:Finished
            (Variables|Default|SetNotInAction true)
            (bind _output_get (Variables|Default|SetTryNumber (+ (Variables|Default|GetTryNumber) 1)))
            (if (== _output_get (Variables|Default|GetTryNumberForNext))
              (Class|PlayerComponent|IncreaseTaskValue _outputpin)
              (CallFunction|GlowifWrong)))))
      (:2
        (Variables|Default|SetTryNumberForNext 3)
        ;[1 1 1] Jour 2+
        (Audio|SpawnSoundAttached "/Game/Sound/Motor.Motor" (Variables|Default|GetMediaSound) "None" "0, 0, 0" "0, 0, 0" "KeepRelativeOffset" false 1.0 1.0 0.0 "/Game/Sound/TestAttenuation.TestAttenuation" 0 :!label _label)
        (bind _displacement_2 (Timeline|Turn_Anim PlayFromStart)
          (:Update
            (Transformation|SetRelativeRotation (Variables|Default|GetManivelle_parent) (Math|Rotator|MakeRotator _roll_2 _displacement_2 _yaw_2) false false))
          (:Finished
            (Variables|Default|SetNotInAction true)
            (bind _output_get_2 (Variables|Default|SetTryNumber (+ (Variables|Default|GetTryNumber) 1)))
            (if (== _output_get_2 (Variables|Default|GetTryNumberForNext))
              (bind _dayvalue_2 (CallFunction|CheckDay CharacterRef))
              (if (== _dayvalue_2 2)
                (bind _soundinstance (Default|Speak (Variables|Ref|GetPlayerRef) "/Game/Sound/Voices/Jour2/Astute/Voice_Astute_J2_4_Cue.Voice_Astute_J2_4_Cue"))
                (EventDispatchers|BindEventtoOnAudioFinished _soundinstance (delegate Custom|CustomEvent_0))
                (else
                  (if (!= _dayvalue_2 6)
                    _
                    (else
                      (bind _returnvalue_2 (Actor|GetActorOfClass "/Game/BP/PrefabLD/Modules/BP_Cabin.BP_Cabin_C"))
                      (bind _output_get_3 (Variables|Default|SetCabine _returnvalue_2))
                      (Transformation|AddActorWorldOffset _output_get_3 "0, 0,-500.000000")
                      (bind _returnvalue_3 (Actor|GetActorOfClass "/Game/BP/PrefabLD/Modules/Cabin.Cabin_C"))
                      (bind _output_get_4 (Variables|Default|SetCabine_Compo _returnvalue_3))
                      (Transformation|AddActorWorldOffset _output_get_4 "0, 0,500.000000")))
                  (Class|PlayerComponent|IncreaseTaskValue _outputpin)
                  (CallFunction|GlowifWrong)))))))
      (:3
        (Variables|Default|SetTryNumberForNext 2 :!label _label_2)
        (goto _label))
      (:6
        (goto _label_2)))))

(fn ConstructionScript
  (bind _returnvalue (Rendering|Material|CreateDynamicMaterialInstance "/Game/Materials/oldMats/M_buttonOutline_Inst.M_buttonOutline_Inst" "None" "None" :!class /Script/Engine.KismetMaterialLibrary))
  (bind _output_get (Variables|Default|SetBodyPaint _returnvalue))
  (Rendering|Material|SetMaterial (Variables|Default|GetOutline) 0 _output_get)
  (bind _returnvalue_2 (Actor|GetActorOfClass "/Game/BP/FirstPerson/FirstPersonCharacter.FirstPersonCharacter_C"))
  (Variables|Ref|SetPlayerRef _returnvalue_2)
  (bind _returnvalue_3 (Actor|GetActorOfClass "/Game/BP/BP_Button_C_Alim.BP_Button_C_Alim_C"))
  (Variables|Ref|SetAlimRef _returnvalue_3))

(fn CheckTaskOrder
  (params (Target :type Actor%20Object%20Reference))
  (bind _returnvalue (Actor|GetComponentbyClass Target "/Script/Dietemna.PlayerComponent"))
  (bind _returnvalue_2 (Class|PlayerComponent|GetTaskValue _returnvalue))
  (return (== _returnvalue_2 (Variables|TaskOrder|GetDayTaskValue)) _returnvalue))

(fn CheckDay
  (params (Chara :type Actor%20Object%20Reference))
  (bind _returnvalue (Actor|GetComponentbyClass Chara "/Script/Dietemna.PlayerComponent"))
  (bind _returnvalue_2 (Class|PlayerComponent|GetDayValue _returnvalue))
  (return _returnvalue_2 _returnvalue))

(fn CheckTaskAbove
  (params (Target :type Actor%20Object%20Reference))
  (bind _returnvalue (Actor|GetComponentbyClass Target "/Script/Dietemna.PlayerComponent"))
  (bind _returnvalue_2 (Class|PlayerComponent|GetTaskValue _returnvalue))
  (return (<= _returnvalue_2 (Variables|TaskOrder|GetDayTaskValue)) _returnvalue))