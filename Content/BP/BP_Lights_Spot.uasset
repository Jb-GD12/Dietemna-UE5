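; Spot light Blueprint that starts dark and toggles on or off through the SwitchOnLight event.
; A FlipFlop plays LightTimeline forward or in reverse, scaling its brightness track by Intensity to fade the light, and clears NotActive when it finishes.
; A day 2 alarm flicker using a looping FadingLight timeline exists but is disconnected, and BeginPlay does nothing.
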(event Custom|SwitchOnLight
  (Utilities|FlowControl|FlipFlop
    (:A
      ;[1 1 1] Change Light color
      (bind _lightbrightnessfloattrack (Timeline|LightTimeline PlayFromStart)
        (:Update
          (Rendering|Components|Light|SetIntensity (Variables|Default|GetSpotLight) (* _lightbrightnessfloattrack (Variables|Light|GetIntensity))))
        (:Finished
          (Variables|Default|SetNotActive false))))
    (:B
      (Timeline|LightTimeline ReverseFromEnd))))

(event EventBeginPlay)

(fn ConstructionScript
  (Rendering|Components|Light|SetIntensity (Variables|Default|GetSpotLight) 0.0))