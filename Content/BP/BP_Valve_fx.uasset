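; Interactable valve Blueprint that turns when used and then releases a smoke effect.
; On Interact, a timeline drives the valve mesh's relative yaw from a scaled curve.
; When the timeline finishes, a P_Smoke emitter spawns at the valve's world location and is stored in FXEmitter.
; The delayed destruction of that emitter is unconnected, so the Blueprint never removes the smoke itself.
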(event EventInteract
  (params (CharacterRef :type Character%20Object%20Reference))
  (bind _valve (Variables|Default|GetValve))
  (bind _relativerotation (Variables|/Script/Engine.SceneComponent|GetRelativeRotation _valve))
  (bind (_roll _pitch) (Math|Rotator|BreakRotator _relativerotation))
  (bind _rotz (Timeline|Timeline_0 Play)
    (:Update
      (Transformation|SetRelativeRotation _valve (Math|Rotator|MakeRotator _roll _pitch (* _rotz 6e+01)) false false))
    (:Finished
      (bind _returnvalue (Effects|SpawnEmitteratLocation "/Game/_StarterContent/Particles/P_Smoke.P_Smoke" (+ (Transformation|GetWorldLocation (Variables|Default|GetValve)) "") (Math|Rotator|MakeRotator 0.0 0.0 0.0)))
      (bind _output_get (Variables|Default|SetFXEmitter _returnvalue)))))

(fn ConstructionScript)