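; An interactive alarm clock button, derived from a parent button Blueprint, that rings until the player turns it off as a task step.
; On BeginPlay it spawns an attached alarm sound on the MediaSound component and keeps a reference to it.
; On Interact it runs the parent logic, then, if the task order check passes, stops the sound, increases the task value and calls GlowIfWrong.
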(event EventBeginPlay
  (bind _returnvalue (Audio|SpawnSoundAttached (Variables|Default|GetSoundCue) (Variables|Default|GetMediaSound) "None" "0, 0, 0" "0, 0, 0" "KeepRelativeOffset" false 1.0 1.0 0.0 "/Game/Sound/NewSoundAttenuation.NewSoundAttenuation" 0))
  (Variables|Default|SetAlarmSound _returnvalue))

(event EventInteract
  (params (CharacterRef :type Character%20Object%20Reference))
  (|CallParentFunction CharacterRef)
  (bind (_returnvalue _outputpin) (CallFunction|CheckTaskOrder CharacterRef))
  (if _returnvalue
    (Audio|Components|Audio|Stop (Variables|Default|GetAlarmSound))
    (Class|PlayerComponent|IncreaseTaskValue _outputpin)
    (CallFunction|GlowifWrong)))

(fn ConstructionScript
  (|CallParentFunction))