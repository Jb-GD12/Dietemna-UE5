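; BP_Door_Sas2 is a hinged metal door that toggles open and closed through its OpenDoor event unless Locked.
; The OpenDoorT timeline drives the door's yaw up to 90 degrees and reverses to close it.
; An opening sound plays on each toggle, and a closing sound when closing finishes.
; Doors set open start rotated via the construction script, and BeginOpen makes their first close reverse from the timeline's end.
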(event Custom|OpenDoor
  (params (Player :type Actor%20Object%20Reference))
  (if (not (Variables|Default|GetLocked))
    (Audio|SpawnSoundAttached "/Game/Sound/FX/Metal-Door-opening.Metal-Door-opening" (Variables|Default|GetMediaSound) "None" "0, 0, 0" "0, 0, 0" "KeepRelativeOffset" false 1.0 1.0 0.0 0 0)
    (if (Variables|Default|GetDoorClosed)
      (Variables|Default|SetDoorClosed false)
      (bind _doorrotatez (Timeline|OpenDoorT Play)
        (:Update
          (Transformation|SetRelativeRotation (Variables|Default|GetDoor) (Math|Rotator|MakeRotator 0.0 0.0 (* _doorrotatez 9e+01)) false false))
        (:Finished
          (if (Variables|Default|GetDoorClosed)
            (Audio|SpawnSoundAttached "/Game/Sound/FX/Metal-Door-closing.Metal-Door-closing" (Variables|Default|GetMediaSound) "None" "0, 0, 0" "0, 0, 0" "KeepRelativeOffset" false 1.0 1.0 0.0 0 0))))
      (else
        (Variables|Default|SetDoorClosed true)
        (if (Variables|Default|GetBeginOpen)
          (Variables|Default|SetBeginOpen false)
          (Timeline|OpenDoorT ReverseFromEnd)
          (else
            (Timeline|OpenDoorT Reverse)))))))

(fn ConstructionScript
  (if (not (Variables|Default|GetDoorClosed))
    (Variables|Default|SetBeginOpen true)
    (Transformation|SetRelativeRotation (Variables|Default|GetDoor) (Math|Rotator|MakeRotator 0.0 0.0 9e+01) false false)))