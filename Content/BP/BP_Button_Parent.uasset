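; Parent Blueprint for pushable buttons that signal whether they match the player's current task.
; Interact plays an attached sound and a timeline that slides the button along Y.
; GlowIfWrong compares the PlayerComponent task value to DayTaskValue, running the Glow2 color timeline in reverse on a match, forward otherwise.
; That timeline drives EmissiveColor on the outline's dynamic material, created in the construction script; an older Glow branch never runs.
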(event Custom|GlowIfWrong
  ;[1 1 1] Glow passe du vert au rouge quand la tâche à été effectué
  (bind _returnvalue (CallFunction|CheckTaskOrder (Game|GetPlayerCharacter 0)))
  (if _returnvalue
    (bind _matcolor (Timeline|Glow2 ReverseFromEnd)
      (:Update
        (Rendering|Material|SetVectorParameterValue (Variables|Default|GetBodyPaint) "EmissiveColor" _matcolor :!class /Script/Engine.MaterialInstanceDynamic)))
    (else
      (Timeline|Glow2 PlayFromStart))))

(event EventInteract
  (params (CharacterRef :type Character%20Object%20Reference))
  ;[1 1 1] Push Anim + Push Sound
  (Audio|SpawnSoundAttached "/Game/Sound/button.button" (Variables|Default|GetMediaSound) "None" "0, 0, 0" "0, 0, 0" "KeepRelativeOffset" false 1.0 1.0 0.0 "/Game/Sound/NewSoundAttenuation.NewSoundAttenuation" 0)
  (bind _displacement (Timeline|Push_anim PlayFromStart)
    (:Update
      (Transformation|SetRelativeLocation (Variables|Default|GetButton) (* "0,-5.000000, 0" _displacement) false false))))

(fn ConstructionScript
  (bind _returnvalue (Rendering|Material|CreateDynamicMaterialInstance "/Game/Materials/M_buttonOutline_Inst.M_buttonOutline_Inst" "None" "None" :!class /Script/Engine.KismetMaterialLibrary))
  (bind _output_get (Variables|Default|SetBodyPaint _returnvalue))
  (Rendering|Material|SetMaterial (Variables|Default|GetOutline) 0 _output_get))

(fn CheckTaskOrder
  (params (Target :type Actor%20Object%20Reference))
  (bind _returnvalue (Actor|GetComponentbyClass Target "/Script/Dietemna.PlayerComponent"))
  (bind _returnvalue_2 (Class|PlayerComponent|GetTaskValue _returnvalue))
  (return (== _returnvalue_2 (Variables|TaskOrder|GetDayTaskValue)) _returnvalue))