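; BP_ColorSwitchButton is an interactable button that switches the color of BP_ColorSwitch actors whose ColorSwitchValue matches its ButtonValue.
; Interact plays the Push_anim timeline, which offsets the button mesh along local Y.
; Every timeline update also checks that the character's PlayerComponent task value equals DayTaskValue, then calls SwitchColor on all matching actors.
; The IncreaseTaskValue call is unconnected, so the button never advances the task.
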(event EventInteract
  (params (CharacterRef :type Character%20Object%20Reference))
  (bind _displacement (Timeline|Push_anim PlayFromStart)
    (:Update
      (Transformation|SetRelativeLocation (Variables|Default|GetButton) (* "0,-5.000000, 0" _displacement) false false)
      (bind (_returnvalue _playercomponent) (|CheckTaskOrder CharacterRef))
      (if _returnvalue
        (bind _outactors (Actor|GetAllActorsOfClass "/Game/BP/BP_ColorSwitch.BP_ColorSwitch_C"))
        (bind _array_element (Utilities|Array|ForEachLoopwithBreak _outactors)
          (:LoopBody
            (if (== (Variables|/Game/BP/BP_ColorSwitch.BP_ColorSwitch_C|GetColorSwitchValue _array_element) (Variables|LinkInstance|GetButtonValue))
              (Default|SwitchColor _array_element))))))))

(fn ConstructionScript)