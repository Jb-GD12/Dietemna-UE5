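; Food dispenser Blueprint that opens a door and pushes out a plate when OpenFoodGiver is called.
; The OpenDoor timeline raises the door by accumulating relative Z offsets, then starts the MovePlate timeline on completion.
; MovePlate adds X linear velocity to the physics-simulated plate each update, then zeroes it and disables physics when finished.
; An unconnected relative-location move for the plate remains unused.
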(event Custom|OpenFoodGiver
  (bind _door (Variables|Default|GetDoor))
  (bind _plate (Variables|Default|GetPlate))
  (bind _displacement (Timeline|OpenDoor PlayFromStart)
    (:Update
      (Transformation|SetRelativeLocation _door (+ (Variables|/Script/Engine.SceneComponent|GetRelativeLocation _door) (* "0,0.000000,2.000000" _displacement)) false false))
    (:Finished
      (bind _forwardplate (Timeline|MovePlate PlayFromStart)
        (:Update
          (Physics|SetPhysicsLinearVelocity _plate (* "5.000000,0.000000,0.000000" _forwardplate) true "None"))
        (:Finished
          (Physics|SetPhysicsLinearVelocity _plate "0, 0, 0" false "None")
          (Physics|SetSimulatePhysics _plate false))))))

(fn ConstructionScript)